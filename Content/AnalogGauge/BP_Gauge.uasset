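; BP_Gauge is an analog gauge actor that displays an insulation reading with a rotating needle.
; Shortly after BeginPlay it casts its parent actor to BP_PanelBase and stops if that fails.
; Objective panels show their CurrentInsulation, while other panels get a random high-range value.
; TurnNeedle maps the value to needle pitch with a Lerp, set once rather than updated on Tick.
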(event EventBeginPlay
  (Utilities|FlowControl|Delay 0.5)
  (bind _asbp_panel_base (Utilities|Casting|CastToBP_PanelBase (Actor|GetParentActor)))
  (if (Variables|/Game/Levels/Level2/Blueprints/Panels/BP_PanelBase.BP_PanelBase_C|GetPanelIsObjective _asbp_panel_base)
    (CallFunction|TurnNeedle (Variables|/Game/Levels/Level2/Blueprints/Panels/BP_PanelBase.BP_PanelBase_C|GetCurrentInsulation _asbp_panel_base))
    (else
      (CallFunction|TurnNeedle (Math|Random|RandomFloatinRange 0.6 0.9)))))

(event Collision|EventActorBeginOverlap
  (params (OtherActor :type Actor%20Object%20Reference)))

(event EventTick
  (params (DeltaSeconds :type Float%20%28single-precision%29)))

(fn ConstructionScript)

(fn TurnNeedle
  (params (Input :type Float%20%28double-precision%29))
  (Transformation|SetRelativeRotation (Variables|Default|GetNeedle) (Math|Rotator|MakeRotator 0.0 (Math|Float|Lerp -55.0 35.0 Input) 0.0) false false))