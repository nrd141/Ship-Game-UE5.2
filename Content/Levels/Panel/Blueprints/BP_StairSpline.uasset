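; BP_StairSpline is a stair trigger that switches the first-person player into and out of spline movement.
; BeginPlay caches the player character after a short delay, and SplineCollision overlaps call BeginSpline or EndSpline for that character.
; These set the character's InSpline flag and SplineRef, toggle its gravity, and set StartTick, which nothing here reads.
; The nodes that snap positions to the spline are disconnected, so this Blueprint moves nothing itself.
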(event OnComponentBeginOverlap(SplineCollision)
  (params (OverlappedComponent :type Primitive%20Component%20Object%20Reference) (OtherActor :type Actor%20Object%20Reference) (OtherComp :type Primitive%20Component%20Object%20Reference) (OtherBodyIndex :type Integer) (bFromSweep :type Boolean) (SweepResult :type Hit%20Result%20Structure%20%28by%20ref%29))
  (if (== OtherActor (Variables|Default|GetAs%20BP%20First%20Person%20Character))
    (CallFunction|BeginSpline)))

(event OnComponentEndOverlap(SplineCollision)
  (params (OverlappedComponent :type Primitive%20Component%20Object%20Reference) (OtherActor :type Actor%20Object%20Reference) (OtherComp :type Primitive%20Component%20Object%20Reference) (OtherBodyIndex :type Integer))
  (if (== OtherActor (Variables|Default|GetAs%20BP%20First%20Person%20Character))
    (CallFunction|EndSpline)))

(event Custom|BeginSpline
  (bind _as_bp_first_person_character (Variables|Default|GetAs%20BP%20First%20Person%20Character))
  (Variables|/Game/Levels/Panel/Blueprints/BP_FirstPersonCharacter.BP_FirstPersonCharacter_C|SetInSpline _as_bp_first_person_character true)
  (Variables|/Game/Levels/Panel/Blueprints/BP_FirstPersonCharacter.BP_FirstPersonCharacter_C|SetSplineRef _as_bp_first_person_character self)
  (Variables|/Script/Engine.CharacterMovementComponent|SetGravityScale (Variables|/Script/Engine.Character|GetCharacterMovement _as_bp_first_person_character) 0.0)
  (Variables|Default|SetStartTick true))

(event Custom|EndSpline
  (bind _as_bp_first_person_character (Variables|Default|GetAs%20BP%20First%20Person%20Character))
  (Variables|/Game/Levels/Panel/Blueprints/BP_FirstPersonCharacter.BP_FirstPersonCharacter_C|SetInSpline _as_bp_first_person_character false)
  (Variables|/Game/Levels/Panel/Blueprints/BP_FirstPersonCharacter.BP_FirstPersonCharacter_C|SetSplineRef _as_bp_first_person_character self)
  (Variables|Default|SetStartTick false)
  (Variables|/Script/Engine.CharacterMovementComponent|SetGravityScale (Variables|/Script/Engine.Character|GetCharacterMovement _as_bp_first_person_character) 1.0))

(event EventBeginPlay
  (Utilities|FlowControl|Delay 1.0)
  (bind _asbp_first_person_character (Utilities|Casting|CastToBP_FirstPersonCharacter (Game|GetPlayerCharacter 0)))
  (Variables|Default|SetAs%20BP%20First%20Person%20Character _asbp_first_person_character))

(fn ConstructionScript)