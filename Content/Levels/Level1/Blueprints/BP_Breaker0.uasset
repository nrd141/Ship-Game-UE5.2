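; Interactable circuit breaker for a fault-finding level, mounted on a BP_PanelBase panel.
; InteractSwitch plays a click, then loses the game if the breaker is critical; other breakers toggle switch rotation and standby material.
; Wrong breakers add to a score penalty.
; The objective breaker drives the panel's LED and gauge; its first find awards penalty-adjusted, floored score and updates the objective text, or wins on the last panel.
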(event EventBeginPlay)

(event Collision|EventActorBeginOverlap
  (params (OtherActor :type Actor%20Object%20Reference)))

(fn ConstructionScript
  (bind _asbp_first_person_game_mode (Utilities|Casting|CastToBP_FirstPersonGameMode (Game|GetGameMode)))
  (Variables|Default|SetAs%20BP%20First%20Person%20Game%20Mode _asbp_first_person_game_mode)
  (bind _asbp_panel_base (Utilities|Casting|CastToBP_PanelBase (Actor|GetParentActor)))
  (Variables|Default|SetAs%20BP%20Panel%20Base _asbp_panel_base))

(fn InteractSwitch
  (bind _returnvalue (Actor|GetAttachParentActor))
  (bind _bp_breaker_switch (Variables|Default|GetBP_Breaker_Switch))
  (bind _cb_st_by_ind_ (Variables|Default|GetCB_st_by_ind_))
  (Audio|PlaySoundatLocation "/Game/SFX/item/circuit-breaker-1-sp-90840.circuit-breaker-1-sp-90840" (Transformation|GetActorLocation) "0, 0, 0" (Math|Random|RandomFloatinRange 0.4 0.5) (Math|Random|RandomFloatinRange 0.9 1.1) 0.0 0 0 0 0)
  (if (Variables|Default|GetIsCritical)
    (bind _asbp_first_person_game_mode (Utilities|Casting|CastToBP_FirstPersonGameMode (Game|GetGameMode)))
    (Variables|/Game/Levels/Panel/Blueprints/BP_FirstPersonGameMode.BP_FirstPersonGameMode_C|SetGameCondition _asbp_first_person_game_mode false)
    (Default|EndGame _asbp_first_person_game_mode)
    (elif (Variables|Default|GetObjective)
      (if (Variables|Default|GetFoundObjective)
        (if (Variables|Default|GetIsOn) :!label _label
          (Transformation|SetRelativeRotation _bp_breaker_switch "0.000000,0.000000,20.000000" false false)
          (Rendering|Material|SetMaterial _cb_st_by_ind_ 0 "/Game/Levels/Level1/Circuit_Breaker_obj/st-by_off.st-by_off")
          (Variables|Default|SetIsOn false)
          (if (Variables|Default|GetObjective)
            (bind _asbp_panel_base (Utilities|Casting|CastToBP_PanelBase _returnvalue))
            (Default|TurnGreen (Variables|/Game/Levels/Level2/Blueprints/Panels/BP_PanelBase.BP_PanelBase_C|GetLEDIndicator _asbp_panel_base))
            (Default|TurnNeedle (Variables|/Game/Levels/Level2/Blueprints/Panels/BP_PanelBase.BP_PanelBase_C|GetGauge _asbp_panel_base) (Math|Random|RandomFloatinRange 0.6 0.9)))
          (else
            (Transformation|SetRelativeRotation _bp_breaker_switch "0.000000,0.000000,-90.000000" false false)
            (Rendering|Material|SetMaterial _cb_st_by_ind_ 0 "/Game/Levels/Level1/Circuit_Breaker_obj/st-by_on.st-by_on")
            (Variables|Default|SetIsOn true)
            (if (Variables|Default|GetObjective)
              (bind _asbp_panel_base_2 (Utilities|Casting|CastToBP_PanelBase _returnvalue))
              (Default|TurnRed (Variables|/Game/Levels/Level2/Blueprints/Panels/BP_PanelBase.BP_PanelBase_C|GetLEDIndicator _asbp_panel_base_2))
              (Default|TurnNeedle (Variables|/Game/Levels/Level2/Blueprints/Panels/BP_PanelBase.BP_PanelBase_C|GetGauge _asbp_panel_base_2) (Math|Random|RandomFloatinRange 0.1 0.2)))))
        (else
          (Transformation|SetRelativeRotation (Variables|Default|GetBP_Breaker_Switch) "0.000000,0.000000,20.000000" false false)
          (Rendering|Material|SetMaterial (Variables|Default|GetCB_st_by_ind_) 0 "/Game/Levels/Level1/Circuit_Breaker_obj/st-by_off.st-by_off")
          (if (Variables|Default|GetObjective)
            (bind _asbp_panel_base_3 (Utilities|Casting|CastToBP_PanelBase (Actor|GetAttachParentActor)))
            (Default|TurnGreen (Variables|/Game/Levels/Level2/Blueprints/Panels/BP_PanelBase.BP_PanelBase_C|GetLEDIndicator _asbp_panel_base_3))
            (Default|TurnNeedle (Variables|/Game/Levels/Level2/Blueprints/Panels/BP_PanelBase.BP_PanelBase_C|GetGauge _asbp_panel_base_3) (Math|Random|RandomFloatinRange 0.6 0.9))
            (Variables|Default|SetFoundObjective true)
            (Audio|PlaySoundatLocation "/Game/SFX/ui/90s-game-ui-7-185100.90s-game-ui-7-185100" (Transformation|GetActorLocation) "0, 0, 0" 1.0 1.0 0.0 0 0 0 0)
            (Development|PrintString (Utilities|String|Append "Fault found in " (Utilities|GetDisplayName (Actor|GetAttachParentActor))))
            (bind _asbp_first_person_game_mode_2 (Utilities|Casting|CastToBP_FirstPersonGameMode (Game|GetGameMode)))
            (bind _asmy_game_instance (Utilities|Casting|CastToMyGameInstance (Game|GetGameInstance)))
            (Variables|/Game/MyGameInstance.MyGameInstance_C|SetObjective _asmy_game_instance "Find The Next Panel")
            (if (<= (- (+ (Variables|/Game/Levels/Panel/Blueprints/BP_FirstPersonGameMode.BP_FirstPersonGameMode_C|GetScore _asbp_first_person_game_mode_2) 100) (Variables|/Game/Levels/Panel/Blueprints/BP_FirstPersonGameMode.BP_FirstPersonGameMode_C|GetTempScore _asbp_first_person_game_mode_2)) 50)
              (Variables|/Game/Levels/Panel/Blueprints/BP_FirstPersonGameMode.BP_FirstPersonGameMode_C|SetScore _asbp_first_person_game_mode_2 50)
              (else
                (Variables|/Game/Levels/Panel/Blueprints/BP_FirstPersonGameMode.BP_FirstPersonGameMode_C|SetScore _asbp_first_person_game_mode_2 (- (+ (Variables|/Game/Levels/Panel/Blueprints/BP_FirstPersonGameMode.BP_FirstPersonGameMode_C|GetScore _asbp_first_person_game_mode_2) 100) (Variables|/Game/Levels/Panel/Blueprints/BP_FirstPersonGameMode.BP_FirstPersonGameMode_C|GetTempScore _asbp_first_person_game_mode_2)))))
            (Variables|/Game/Levels/Panel/Blueprints/BP_FirstPersonGameMode.BP_FirstPersonGameMode_C|SetTempScore _asbp_first_person_game_mode_2 0)
            (bind _asbp_panel_base_4 (Utilities|Casting|CastToBP_PanelBase (Actor|GetAttachParentActor)))
            (if (Variables|/Game/Levels/Level2/Blueprints/Panels/BP_PanelBase.BP_PanelBase_C|GetIsLast _asbp_panel_base_4)
              (Development|PrintString "Root fault is found")
              (bind _asbp_first_person_game_mode_3 (Utilities|Casting|CastToBP_FirstPersonGameMode (Game|GetGameMode)))
              (Variables|/Game/Levels/Panel/Blueprints/BP_FirstPersonGameMode.BP_FirstPersonGameMode_C|SetGameCondition _asbp_first_person_game_mode_3 true)
              (Default|EndGame _asbp_first_person_game_mode_3)
              (else
                (goto _label))))))
      (else
        (bind _asbp_first_person_game_mode_4 (Utilities|Casting|CastToBP_FirstPersonGameMode (Game|GetGameMode)))
        (Variables|/Game/Levels/Panel/Blueprints/BP_FirstPersonGameMode.BP_FirstPersonGameMode_C|SetTempScore _asbp_first_person_game_mode_4 (+ (Variables|/Game/Levels/Panel/Blueprints/BP_FirstPersonGameMode.BP_FirstPersonGameMode_C|GetTempScore _asbp_first_person_game_mode_4) 5))
        (goto _label)))))