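; Confirm-button widget actor attached to a fault-finding panel that checks whether the player's checkbox selection matches the panel's solution.
; ConfirmFunction casts the parent to BP_PanelLevel1 on level1 or BP_PanelBase elsewhere and compares the arrays, adding a TempScore penalty on mismatch.
; The first match plays a sound, updates the objective and adds penalty-reduced points to Score with a floor.
; A match on the last panel ends the game.
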(event EventBeginPlay)

(event Collision|EventActorBeginOverlap
  (params (OtherActor :type Actor%20Object%20Reference)))

(event EventTick
  (params (DeltaSeconds :type Float%20%28single-precision%29)))

(fn ConstructionScript)

(fn ConfirmFunction
  (bind _returnvalue (Actor|GetAttachParentActor))
  (bind _returnvalue_2 (Game|GetCurrentLevelName true))
  (if (Utilities|Enum|Equal(Enum) _returnvalue_2 "level1")
    (bind _asbp_panel_level_1 (Utilities|Casting|CastToBP_PanelLevel1 (Actor|GetAttachParentActor)))
    (Utilities|Casting|CastToConfirmButtonWidget (UserInterface|GetWidget (Variables|Default|GetWidget)))
    (bind _asbp_first_person_game_mode (Utilities|Casting|CastToBP_FirstPersonGameMode (Game|GetGameMode)))
    (if (Utilities|Array|Identical (Variables|/Game/Levels/Level1/Blueprints/BP_PanelLevel1.BP_PanelLevel1_C|GetCheckboxButtonsArray _asbp_panel_level_1) (Variables|/Game/Levels/Level1/Blueprints/BP_PanelLevel1.BP_PanelLevel1_C|GetCheckboxSolutionsArray _asbp_panel_level_1))
      (if (not (Variables|Default|GetFoundObjective)) :!label _label
        (Variables|Default|SetFoundObjective true)
        (Audio|PlaySoundatLocation "/Game/SFX/ui/90s-game-ui-7-185100.90s-game-ui-7-185100" (Transformation|GetActorLocation) "0, 0, 0" 1.0 1.0 0.0 0 0 0 0)
        (Development|PrintString (Utilities|String|Append "Fault found in " (Utilities|GetDisplayName (Actor|GetAttachParentActor))))
        (bind _asbp_first_person_game_mode_2 (Utilities|Casting|CastToBP_FirstPersonGameMode (Game|GetGameMode)))
        (bind _asmy_game_instance (Utilities|Casting|CastToMyGameInstance (Game|GetGameInstance)))
        (Variables|/Game/MyGameInstance.MyGameInstance_C|SetObjective _asmy_game_instance "Find The Next Panel")
        (if (<= (- (+ (Variables|/Game/Levels/Panel/Blueprints/BP_FirstPersonGameMode.BP_FirstPersonGameMode_C|GetScore _asbp_first_person_game_mode_2) 100) (Variables|/Game/Levels/Panel/Blueprints/BP_FirstPersonGameMode.BP_FirstPersonGameMode_C|GetTempScore _asbp_first_person_game_mode_2)) 50)
          (Variables|/Game/Levels/Panel/Blueprints/BP_FirstPersonGameMode.BP_FirstPersonGameMode_C|SetScore _asbp_first_person_game_mode_2 50)
          (else
            (Variables|/Game/Levels/Panel/Blueprints/BP_FirstPersonGameMode.BP_FirstPersonGameMode_C|SetScore _asbp_first_person_game_mode_2 (- (+ (Variables|/Game/Levels/Panel/Blueprints/BP_FirstPersonGameMode.BP_FirstPersonGameMode_C|GetScore _asbp_first_person_game_mode_2) 100) (Variables|/Game/Levels/Panel/Blueprints/BP_FirstPersonGameMode.BP_FirstPersonGameMode_C|GetTempScore _asbp_first_person_game_mode_2)))))
        (Variables|/Game/Levels/Panel/Blueprints/BP_FirstPersonGameMode.BP_FirstPersonGameMode_C|SetTempScore _asbp_first_person_game_mode_2 0)
        (bind _returnvalue_3 (Game|GetCurrentLevelName true))
        (if (Utilities|Enum|Equal(Enum) _returnvalue_3 "level1")
          (bind _asbp_panel_level_1_2 (Utilities|Casting|CastToBP_PanelLevel1 _returnvalue))
          (if (Variables|/Game/Levels/Level1/Blueprints/BP_PanelLevel1.BP_PanelLevel1_C|GetIsLast _asbp_panel_level_1_2)
            (Development|PrintString "Root fault is found")
            (bind _asbp_first_person_game_mode_3 (Utilities|Casting|CastToBP_FirstPersonGameMode (Game|GetGameMode)))
            (Variables|/Game/Levels/Panel/Blueprints/BP_FirstPersonGameMode.BP_FirstPersonGameMode_C|SetGameEnded _asbp_first_person_game_mode_3 true)
            (Variables|/Game/Levels/Panel/Blueprints/BP_FirstPersonGameMode.BP_FirstPersonGameMode_C|SetGameCondition _asbp_first_person_game_mode_3 true)
            (Default|EndGame _asbp_first_person_game_mode_3))
          (else
            (bind _asbp_panel_base (Utilities|Casting|CastToBP_PanelBase _returnvalue))
            (if (Variables|/Game/Levels/Level2/Blueprints/Panels/BP_PanelBase.BP_PanelBase_C|GetIsLast _asbp_panel_base)
              (Development|PrintString "Root fault is found")
              (bind _asbp_first_person_game_mode_4 (Utilities|Casting|CastToBP_FirstPersonGameMode (Game|GetGameMode)))
              (Variables|/Game/Levels/Panel/Blueprints/BP_FirstPersonGameMode.BP_FirstPersonGameMode_C|SetGameEnded _asbp_first_person_game_mode_4 true)
              (Variables|/Game/Levels/Panel/Blueprints/BP_FirstPersonGameMode.BP_FirstPersonGameMode_C|SetGameCondition _asbp_first_person_game_mode_4 true)
              (Default|EndGame _asbp_first_person_game_mode_4)))))
      (else
        (Variables|/Game/Levels/Panel/Blueprints/BP_FirstPersonGameMode.BP_FirstPersonGameMode_C|SetTempScore _asbp_first_person_game_mode (+ (Variables|/Game/Levels/Panel/Blueprints/BP_FirstPersonGameMode.BP_FirstPersonGameMode_C|GetTempScore _asbp_first_person_game_mode) 10))))
    (else
      (bind _asbp_panel_base_2 (Utilities|Casting|CastToBP_PanelBase (Actor|GetAttachParentActor)))
      (Utilities|Casting|CastToConfirmButtonWidget (UserInterface|GetWidget (Variables|Default|GetWidget)))
      (bind _asbp_first_person_game_mode_5 (Utilities|Casting|CastToBP_FirstPersonGameMode (Game|GetGameMode)))
      (if (Utilities|Array|Identical (Variables|/Game/Levels/Level2/Blueprints/Panels/BP_PanelBase.BP_PanelBase_C|GetCheckboxButtonsArray _asbp_panel_base_2) (Variables|/Game/Levels/Level2/Blueprints/Panels/BP_PanelBase.BP_PanelBase_C|GetCheckboxSolutionsArray _asbp_panel_base_2))
        (goto _label)
        (else
          (Variables|/Game/Levels/Panel/Blueprints/BP_FirstPersonGameMode.BP_FirstPersonGameMode_C|SetTempScore _asbp_first_person_game_mode_5 (+ (Variables|/Game/Levels/Panel/Blueprints/BP_FirstPersonGameMode.BP_FirstPersonGameMode_C|GetTempScore _asbp_first_person_game_mode_5) 10)))))))