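; BP_Door_02 is an interactable animated metal door for Level1 that opens and closes with sound.
; InteractDoor toggles IsOpened, playing the matching open or close animation on the skeletal mesh and a sound cue at the door's location.
; Box overlap applies an outline overlay material as a highlight; ending overlap sets the overlay to the door material rather than clearing it.
; Nothing in this Blueprint calls InteractDoor, and the overlaps do not filter the overlapping actor.
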(event OnComponentBeginOverlap(Box)
  (params (OverlappedComponent :type Primitive%20Component%20Object%20Reference) (OtherActor :type Actor%20Object%20Reference) (OtherComp :type Primitive%20Component%20Object%20Reference) (OtherBodyIndex :type Integer) (bFromSweep :type Boolean) (SweepResult :type Hit%20Result%20Structure%20%28by%20ref%29))
  (Rendering|Material|SetOverlayMaterial (Variables|Default|GetSK_Door_02_Anim) "/Game/Levels/Level1/Material/M_PP_Outline.M_PP_Outline" :!class /Script/Engine.MeshComponent))

(event OnComponentEndOverlap(Box)
  (params (OverlappedComponent :type Primitive%20Component%20Object%20Reference) (OtherActor :type Actor%20Object%20Reference) (OtherComp :type Primitive%20Component%20Object%20Reference) (OtherBodyIndex :type Integer))
  (Rendering|Material|SetOverlayMaterial (Variables|Default|GetSK_Door_02_Anim) "/Game/Levels/Level1/Material/M_Door_02.M_Door_02" :!class /Script/Engine.MeshComponent))

(event Collision|EventActorBeginOverlap
  (params (OtherActor :type Actor%20Object%20Reference)))

(event EventTick
  (params (DeltaSeconds :type Float%20%28single-precision%29)))

(fn ConstructionScript)

(fn InteractDoor
  (bind _returnvalue (Transformation|GetActorLocation))
  (bind _sk_door_02_anim (Variables|Default|GetSK_Door_02_Anim))
  (if (Variables|Default|GetIsOpened)
    (Components|Animation|PlayAnimation _sk_door_02_anim "/Game/Levels/Level1/Skeletal_Mesh/SM_Door_02_Anim_Anim_ArmatureDoor_Door_02_Close.SM_Door_02_Anim_Anim_ArmatureDoor_Door_02_Close" false)
    (Audio|PlaySoundatLocation "/Game/SFX/item/closing-metal-door-44280_Cue.closing-metal-door-44280_Cue" _returnvalue "0, 0, 0" 1.0 1.0 0.0 0 0 0 0)
    (Variables|Default|SetIsOpened false)
    (else
      (Components|Animation|PlayAnimation _sk_door_02_anim "/Game/Levels/Level1/Skeletal_Mesh/SM_Door_02_Anim_Anim_ArmatureDoor_Door_02_Open.SM_Door_02_Anim_Anim_ArmatureDoor_Door_02_Open" false)
      (Audio|PlaySoundatLocation "/Game/SFX/item/opening-metal-door-98518_Cue.opening-metal-door-98518_Cue" _returnvalue "0, 0, 0" 1.0 1.0 0.0 0 0 0 0)
      (Variables|Default|SetIsOpened true))))