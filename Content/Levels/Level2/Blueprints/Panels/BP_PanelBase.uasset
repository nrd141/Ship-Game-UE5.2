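; Base electrical panel for a Level 2 fault-finding puzzle, with eight breakers, matching checkbox widgets, an LED indicator and a gauge.
; Construction caches placeholder transforms, then BeginPlay spawns and attaches breakers and checkboxes, randomizes high insulation levels and finds the indicator child actors.
; SetRandomObjective marks one breaker as the solution with low insulation, then recurses into its linked NextPanel until the last panel, forming a random fault path.
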(event EventBeginPlay
  (for _index (range 0 7)
    (|SetBy-RefVar (Utilities|Array|Get(acopy) (Variables|Default|GetInsulationLevel0) _index) (Math|Random|RandomFloatinRange 0.6 0.9))
    (|SetBy-RefVar (Utilities|Array|Get(acopy) (Variables|Default|GetInsulationLevel1) _index) (Math|Random|RandomFloatinRange 0.6 0.9))
    (bind _returnvalue (Game|SpawnActorfromClass "/Game/Levels/Level1/Blueprints/BP_Breaker0.BP_Breaker0_C" (Utilities|Array|Get(acopy) (Variables|Default|GetSpawn%20Transform) _index) "Undefined" "MultiplyWithRoot" 0 (Utilities|Array|Get(acopy) (Variables|Default|GetNextPanelArray) _index) false false false 0))
    (Variables|/Game/Levels/Level1/Blueprints/BP_Breaker0.BP_Breaker0_C|SetSwitchIndex _returnvalue _index)
    (Transformation|AttachActorToActor _returnvalue self "None" "KeepWorld" "KeepWorld" "KeepWorld" true)
    (Utilities|Array|Add (Variables|Default|GetBreakerArray) _returnvalue)
    (bind _returnvalue_2 (Game|SpawnActorfromClass "/Game/Levels/Level1/Blueprints/BP_SwitchButtonWidget.BP_SwitchButtonWidget_C" (Utilities|Array|Get(acopy) (Variables|Default|GetCheckbox%20Spawn%20Transform) _index) "Undefined" "MultiplyWithRoot" 0 0))
    (Transformation|AttachActorToActor _returnvalue_2 self "None" "KeepWorld" "KeepWorld" "KeepWorld" true)
    (Utilities|Array|Add (Variables|Default|GetCheckboxArray) _returnvalue_2)
    (Variables|/Game/Levels/Level1/Blueprints/BP_SwitchButtonWidget.BP_SwitchButtonWidget_C|SetButtonIndex _returnvalue_2 _index))
  (for _array_element (Actor|GetComponentsByClass "/Script/Engine.ChildActorComponent")
    (bind _asbp_ledindicator (Utilities|Casting|CastToBP_LEDIndicator (Variables|/Script/Engine.ChildActorComponent|GetChildActor _array_element))
      (:then
        (Variables|Default|SetLEDIndicator _asbp_ledindicator))
      (:CastFailed
        (bind _asbp_gauge (Utilities|Casting|CastToBP_Gauge (Variables|/Script/Engine.ChildActorComponent|GetChildActor _array_element)))
        (Variables|Default|SetGauge _asbp_gauge)))))

(event Collision|EventActorBeginOverlap
  (params (OtherActor :type Actor%20Object%20Reference)))

(event EventTick
  (params (DeltaSeconds :type Float%20%28single-precision%29)))

(fn ConstructionScript
  (CallFunction|InitTransform))

(fn SetRandomObjective
  (bind _returnvalue (Math|Random|RandomFloatinRange 0.1 0.2))
  (bind _breakerarray (Variables|Default|GetBreakerArray))
  (bind _output_get (Variables|Default|SetRandomInt (Math|Random|RandomIntegerinRange 0 (- (Utilities|Array|Length _breakerarray) 1))))
  (Utilities|Array|SetArrayElem (Variables|Default|GetCheckboxSolutionsArray) _output_get true)
  (Variables|/Game/Levels/Level1/Blueprints/BP_Breaker0.BP_Breaker0_C|SetObjective (Utilities|Array|Get(acopy) _breakerarray _output_get) true)
  (bind _output_get_2 (Variables|Default|SetObjectiveBreaker (Utilities|Array|Get(acopy) _breakerarray _output_get)))
  (|SetBy-RefVar (Utilities|Array|Get(acopy) (Variables|Default|GetInsulationLevel0) _output_get) _returnvalue)
  (Variables|Default|SetCurrentInsulation _returnvalue)
  (Variables|Default|SetPanelIsObjective true)
  (if (not (Variables|Default|GetIsLast))
    (bind _output_get_3 (Variables|/Game/Levels/Level1/Blueprints/BP_Breaker0.BP_Breaker0_C|SetNextPanel _output_get_2 (Utilities|Array|Get(acopy) (Variables|Default|GetNextPanelArray) _output_get)))
    (CallFunction|SetRandomObjective _output_get_3)))

(fn InitTransform
  (bind _spawn_transform (Variables|Default|GetSpawn%20Transform))
  (bind _checkbox_spawn_transform (Variables|Default|GetCheckbox%20Spawn%20Transform))
  (Utilities|Array|Add _spawn_transform (Transformation|GetWorldTransform (Variables|Default|GetSwitch0)))
  (Utilities|Array|Add _spawn_transform (Transformation|GetWorldTransform (Variables|Default|GetSwitch1)))
  (Utilities|Array|Add _spawn_transform (Transformation|GetWorldTransform (Variables|Default|GetSwitch2)))
  (Utilities|Array|Add _spawn_transform (Transformation|GetWorldTransform (Variables|Default|GetSwitch3)))
  (Utilities|Array|Add _spawn_transform (Transformation|GetWorldTransform (Variables|Default|GetSwitch4)))
  (Utilities|Array|Add _spawn_transform (Transformation|GetWorldTransform (Variables|Default|GetSwitch5)))
  (Utilities|Array|Add _spawn_transform (Transformation|GetWorldTransform (Variables|Default|GetSwitch6)))
  (Utilities|Array|Add _spawn_transform (Transformation|GetWorldTransform (Variables|Default|GetSwitch7)))
  (Utilities|Array|Add _checkbox_spawn_transform (Transformation|GetWorldTransform (Variables|Default|GetCheckbox0)))
  (Utilities|Array|Add _checkbox_spawn_transform (Transformation|GetWorldTransform (Variables|Default|GetCheckbox1)))
  (Utilities|Array|Add _checkbox_spawn_transform (Transformation|GetWorldTransform (Variables|Default|GetCheckbox2)))
  (Utilities|Array|Add _checkbox_spawn_transform (Transformation|GetWorldTransform (Variables|Default|GetCheckbox3)))
  (Utilities|Array|Add _checkbox_spawn_transform (Transformation|GetWorldTransform (Variables|Default|GetCheckbox4)))
  (Utilities|Array|Add _checkbox_spawn_transform (Transformation|GetWorldTransform (Variables|Default|GetCheckbox5)))
  (Utilities|Array|Add _checkbox_spawn_transform (Transformation|GetWorldTransform (Variables|Default|GetCheckbox6)))
  (Utilities|Array|Add _checkbox_spawn_transform (Transformation|GetWorldTransform (Variables|Default|GetCheckbox7))))